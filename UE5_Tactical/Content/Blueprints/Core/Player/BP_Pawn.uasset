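; BP_Pawn is a camera pawn with planar movement, spring-arm zoom and yaw rotation while the middle mouse button is held.
; Input axes only update desired location, rotation and arm length, with movement flattened to the horizontal plane along the actor's facing.
; Tick eases the actor and spring arm toward those targets with interpolation.
; Zoom is clamped, and below a threshold distance it also drives pitch, so the view angle changes when zooming in close.
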(event EventTick
  (params (DeltaSeconds :type Float%20%28single-precision%29))
  (Variables|Default|SetDelta%20Seconds DeltaSeconds)
  (Variables|/Script/Engine.SpringArmComponent|SetTargetArmLength (Variables|Default|GetSpring%20Arm) (Math|Interpolation|FInterpTo (Variables|/Script/Engine.SpringArmComponent|GetTargetArmLength (Variables|Default|GetSpring%20Arm)) (Variables|Default|GetZoom_Desired) (Variables|Default|GetDelta%20Seconds) 2.0))
  (Transformation|SetActorLocation (Math|Interpolation|VInterpTo (Transformation|GetActorLocation) (Variables|Default|GetLocation_Desired) (Variables|Default|GetDelta%20Seconds) 0.0) false false)
  (Transformation|SetActorRotation (Math|Interpolation|RInterpTo (Transformation|GetActorRotation) (Variables|Default|GetRotation_Desired) (Variables|Default|GetDelta%20Seconds) 5.0)))

(event EventBeginPlay
  (Variables|Default|SetLocation_Desired (Transformation|GetActorLocation))
  (Variables|Default|SetZoom_Desired (Variables|/Script/Engine.SpringArmComponent|GetTargetArmLength (Variables|Default|GetSpring%20Arm)))
  (Variables|Default|SetRotation_Desired (Transformation|GetActorRotation)))

(event Input|ActionEvents|InputActionAction_Middle_Mouse_Button
  (params (Key :type Key%20Structure :default "None"))
  (:Pressed
    (Variables|Default|SetMiddle_Mouse_Button_Pressed true))
  (:Released
    (Variables|Default|SetMiddle_Mouse_Button_Pressed false)))

(event Input|AxisEvents|InputAxisInput_Axis_Zoom
  (params (AxisValue :type Float%20%28single-precision%29))
  (Variables|Default|SetZoom_Desired (Math|Float|Clamp(Float) (+ (Variables|Default|GetZoom_Desired) (* AxisValue 6e+01)) (Variables|Default|GetMIN_ZOOM) (Variables|Default|GetMAX_ZOOM)))
  (if (> (Variables|Default|GetZoom_Desired) (Variables|Default|GetMIN_ZOOM))
    (if (<= (Variables|Default|GetZoom_Desired) (Variables|Default|GetZOOM_ANGLE_MAX_DISTANCE))
      (Variables|Default|SetRotation_Desired (Math|Rotator|MakeRotator 0.0 (Math|Float|Clamp(Float) (/ (- (Variables|Default|GetZOOM_ANGLE_MAX_DISTANCE) (Variables|Default|GetZoom_Desired)) (/ (- (Variables|Default|GetZOOM_ANGLE_MAX_DISTANCE) (Variables|Default|GetMIN_ZOOM)) (Variables|Default|GetMAX_ROTATION_PITCH))) 0.0 (Variables|Default|GetMAX_ROTATION_PITCH)) (.yaw (Variables|Default|GetRotation_Desired)))))))

(event Input|AxisEvents|InputAxisInput_Axis_Forward
  (params (AxisValue :type Float%20%28single-precision%29))
  (bind _returnvalue (Transformation|GetActorForwardVector))
  (Variables|Default|SetForward_Input (* AxisValue 15.0))
  (Variables|Default|SetLocation_Desired (+ (Variables|Default|GetLocation_Desired) (* (Variables|Default|GetForward_Input) (Math|Vector|MakeVector (.x _returnvalue) (.y _returnvalue) 0.0)))))

(event Input|AxisEvents|InputAxisInput_Axis_Right
  (params (AxisValue :type Float%20%28single-precision%29))
  (bind _returnvalue (Transformation|GetActorRightVector))
  (Variables|Default|SetRight_Input (* AxisValue 15.0))
  (Variables|Default|SetLocation_Desired (+ (Variables|Default|GetLocation_Desired) (* (Variables|Default|GetRight_Input) (Math|Vector|MakeVector (.x _returnvalue) (.y _returnvalue) 0.0)))))

(event Input|AxisEvents|InputAxisInput_Axis_Rotation
  (params (AxisValue :type Float%20%28single-precision%29))
  (if (Variables|Default|GetMiddle_Mouse_Button_Pressed)
    (Variables|Default|SetRotation_Desired (Math|Rotator|MakeRotator 0.0 (.pitch (Variables|Default|GetRotation_Desired)) (.yaw (Math|Rotator|CombineRotators (Variables|Default|GetRotation_Desired) (Math|Rotator|MakeRotator 0.0 0.0 (* AxisValue 2.0))))))))

(fn ConstructionScript)